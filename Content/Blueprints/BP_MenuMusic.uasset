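; BP_MenuMusic is a background music player, named for the menu, that plays random C418 tracks on its Audio component.
; After an initial delay on BeginPlay, it loops: pick a random track, set the sound, play it, then wait a fixed interval regardless of track length.
; Repeats are possible, and RandomInteger(3) only yields 0–2, so the fourth track, Wet Hands, is never selected.
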(event `self.ReceiveBeginPlay`
  (bind _audio (`self.Audio`))
  (`KismetSystemLibrary.Delay` 20.0)
  (switch `int` (`KismetMathLibrary.RandomInteger` 3) :!label _label
    (:`0`
      (`AudioComponent.SetSound` _audio "/Game/Assets/Sounds/C418_-_Clark_30921662.C418_-_Clark_30921662"))
    (:`1`
      (`AudioComponent.SetSound` _audio "/Game/Assets/Sounds/C418_-_Haggstrom_30921643.C418_-_Haggstrom_30921643"))
    (:`2`
      (`AudioComponent.SetSound` _audio "/Game/Assets/Sounds/C418_-_Key_30921622.C418_-_Key_30921622"))
    (:`3`
      (`AudioComponent.SetSound` _audio "/Game/Assets/Sounds/C418_-_Wet_Hands_30921656.C418_-_Wet_Hands_30921656")))
  (`AudioComponent.Play` (`self.Audio`) 0.0)
  (`KismetSystemLibrary.Delay` 400.0)
  (goto _label))

(fn `UserConstructionScript`)