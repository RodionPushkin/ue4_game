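; Firearm weapon Blueprint that fires BP_Bullet projectiles and manages magazine reloads from reserve ammo.
; UseWeapon traces from the player camera along the owner's forward vector, then spawns a bullet at the muzzle aimed at the result.
; A loop paced by UseRate sends the attached weapon's muzzle transform through ServerSetMuzzle.
; An empty magazine sets Reloading, whose OnRep starts an authority-side timer that refills using the class-default magazine size.
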(event `ServerSetMuzzle`
  (params (ClientMuzzleLocation :type "Transform Structure"))
  (set `self.ClientMuzzleLocation` ClientMuzzleLocation))

(event `SetMuzzleTransform`
  (params (Character :type "/Game/Blueprints/Player/Game/BP_PlayerCharacter Object Reference"))
  (for _array_element (`self.GetAttachedActors` Character true)
    (bind _asbp_fire_weapon (cast `/Game/Blueprints/Weapons/BP_FireWeapon` _array_element))
    (bind _muzzle (`/Game/Blueprints/Weapons/BP_FireWeapon.Muzzle` _asbp_fire_weapon))
    (bind _output_get (set `self.ClientMuzzleLocation` (`KismetMathLibrary.MakeTransform` (`SceneComponent.K2_GetComponentLocation` _muzzle) (`SceneComponent.K2_GetComponentRotation` _muzzle))))
    (`self.ServerSetMuzzle` _output_get)))

(event `self.ReceiveBeginPlay`
  (`parent.ReceiveBeginPlay`)
  (bind _asbp_player_character (cast `/Game/Blueprints/Player/Game/BP_PlayerCharacter` (`self.GetInstigator`)))
  (`KismetSystemLibrary.Delay` (`self.UseRate`) :!label _label)
  (`self.SetMuzzleTransform` _asbp_player_character)
  (goto _label))

(event `self.StopRateDelay`
  (`parent.StopRateDelay`))

(event `DEBUG`
  (params (Start :type "Vector Structure") (End :type "Vector Structure") (Hit :type "Vector Structure")))

(fn `GetFireTrace`
  (returns (Hit :type "HitResult Structure") (ReturnValue :type Boolean))
  (bind _asbp_player_character (cast `/Game/Blueprints/Player/Game/BP_PlayerCharacter` (`self.GetInstigator`))
    (:`then`
      (bind _returnvalue (`SceneComponent.K2_GetComponentLocation` (`/Game/Blueprints/Player/Game/BP_PlayerCharacter.Camera` _asbp_player_character)))
      (bind (_outhit _returnvalue_2) (`KismetSystemLibrary.LineTraceSingle` _returnvalue (+ _returnvalue (* (`self.GetActorForwardVector` (`self.GetOwner`)) 10000.0)) "TraceTypeQuery1" false (`|MakeArray` self (`self.GetInstigator`) :!type "Actor Object Reference")))
      (bind (_bblockinghit _binitialoverlap _time _distance _location _impactpoint _normal _impactnormal _physmat _hitactor _hitcomponent _hitbonename _hititem _faceindex _tracestart _traceend) (`GameplayStatics.BreakHitResult` _outhit))
      (`self.DEBUG` _tracestart _traceend _impactpoint)
      (return _outhit _returnvalue_2))
    (:`CastFailed`
      (return (struct) false))))

(fn `OnRep_Reloading`
  (`/Engine/EditorBlueprintResources/ActorMacros.Switch Has Authority`
    (:`Authority`
      (if (and (`self.Reloading`) (not (`self.FireActive`)))
        (`KismetSystemLibrary.K2_SetTimer` null "ReloadFiniched" (`self.ReloadTime`))))))

(fn `ReloadFiniched`
  (bind _totalammo (`self.TotalAmmo`))
  (bind (_ammobeforereload _clientmuzzlelocation _currentammo) (defaults `Object` (`GameplayStatics.GetObjectClass` self)))
  (bind _returnvalue (- (`.CurrentAmmo` (defaults `Object` (`GameplayStatics.GetObjectClass` self))) (`self.CurrentAmmo`)))
  (set `self.Reloading` false)
  (if (and (> (`self.TotalAmmo`) 0) (not (>= (`self.CurrentAmmo`) (`.CurrentAmmo` (defaults `Object` (`GameplayStatics.GetObjectClass` self))))))
    (if (== (`self.AmmoBeforeReload`) (`self.CurrentAmmo`))
      (if (and (> (`self.CurrentAmmo`) 0) (not (`self.FireActive`)))
        (if (> _totalammo 0)
          (set `self.TotalAmmo` (- _totalammo _returnvalue))
          (set `self.CurrentAmmo` (+ _returnvalue (`self.CurrentAmmo`))))
        (elif (> (`self.TotalAmmo`) _currentammo)
          (set `self.CurrentAmmo` _currentammo)
          (set `self.TotalAmmo` (- (`self.TotalAmmo`) _currentammo))
          (else
            (set `self.CurrentAmmo` (`self.TotalAmmo`))
            (set `self.TotalAmmo` 0)))))))

(fn `SpawnBullet`
  (params (Hit :type "HitResult Structure") (out :type Boolean))
  (bind (_bblockinghit _binitialoverlap _time _distance _location _impactpoint _normal _impactnormal _physmat _hitactor _hitcomponent _hitbonename _hititem _faceindex _tracestart _traceend) (`GameplayStatics.BreakHitResult` Hit))
  (bind _returnvalue (`self.GetInstigator`))
  (bind _returnvalue_2 (`self.GetInstigator`))
  (bind _location_2 (.location (`self.ClientMuzzleLocation`)))
  (if out
    (`|SpawnActorFromClass` "/Game/Blueprints/Weapons/Bullets/BP_Bullet.BP_Bullet_C" (`KismetMathLibrary.MakeTransform` _location_2 (`KismetMathLibrary.FindLookAtRotation` _location_2 _location)) "AlwaysSpawn" "OverrideRootScale" (`Pawn.GetController` _returnvalue_2) _returnvalue_2)
    (else
      (`|SpawnActorFromClass` "/Game/Blueprints/Weapons/Bullets/BP_Bullet.BP_Bullet_C" (`KismetMathLibrary.MakeTransform` _location_2 (`KismetMathLibrary.FindLookAtRotation` _location_2 _traceend)) "AlwaysSpawn" "OverrideRootScale" (`Pawn.GetController` _returnvalue) _returnvalue)))
  (return))

(fn `UserConstructionScript`
  (`parent.UserConstructionScript`))

(fn `UseWeapon`
  (returns (Used :type Boolean))
  (bind _used (`parent.UseWeapon`))
  (if _used
    (bind (_hit _returnvalue) (`self.GetFireTrace`))
    (bind _asbp_player_character (cast `/Game/Blueprints/Player/Game/BP_PlayerCharacter` (`self.GetInstigator`)))
    (`/Game/Blueprints/Player/Game/BP_PlayerCharacter.PlayFireEffects` _asbp_player_character)
    (`self.SpawnBullet` _hit _returnvalue)
    (return true)
    (elif (and (> (`self.TotalAmmo`) 0) (<= (`self.CurrentAmmo`) 0))
      (set `self.Reloading` true)
      (return false)
      (else
        (return false)))))