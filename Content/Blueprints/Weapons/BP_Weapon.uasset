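; BP_Weapon is a weapon actor that handles ammo, use rate and automatic fire, with no projectile, trace or damage logic of its own.
; UseWeapon spends ammo and starts a cooldown timer if AbleToUseWeapon finds ammo, no cooldown and the instigating BP_PlayerCharacter's Speed at most 600.
; For Auto weapons, StopRateDelay calls UseWeapon again when the cooldown ends, until StopUseWeapon or a failed check clears FireActive.
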(fn `AbleToUseWeapon`
  (returns (Out :type Boolean))
  (bind _asbp_player_character (cast `/Game/Blueprints/Player/Game/BP_PlayerCharacter` (`self.GetInstigator`)))
  (return (and (> (`self.CurrentAmmo`) 0) (not (`self.UseFreezedByRate`)) (not (> (`/Game/Blueprints/Player/Game/BP_PlayerCharacter.Speed` _asbp_player_character) 600.0)))))

(fn `StopRateDelay`
  (set `self.UseFreezedByRate` false)
  (if (and (`self.Auto`) (`self.FireActive`))
    (`self.UseWeapon`)))

(fn `StopUseWeapon`
  (set `self.FireActive` false))

(fn `UserConstructionScript`)

(fn `UseWeapon`
  (returns (Used :type Boolean))
  (if (`self.AbleToUseWeapon`)
    (`/Engine/EditorBlueprintResources/StandardMacros.DecrementInt` (`self.CurrentAmmo`)
      (:`  `
        (`KismetSystemLibrary.K2_SetTimer` null "StopRateDelay" (`self.UseRate`))
        (set `self.UseFreezedByRate` true)
        (if (`self.Auto`)
          (set `self.FireActive` true))
        (return true)))
    (else
      (set `self.FireActive` false)
      (return false))))