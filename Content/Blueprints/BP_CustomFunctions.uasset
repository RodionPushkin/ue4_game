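; BP_CustomFunctions is a set of shared helpers for debug printing, API URL lookup and persisting the user's token and sensitivity.
; DebugText prints with a given color and duration, or adds a red error prefix, while RequestToApi simply returns DefApiUrl without sending a request.
; Save functions load or create BP_SaveGame in one shared slot, change one field and write it back.
; Load functions return defaults when no save exists.
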(fn `DebugText`
  (params (InString :type String :default "print Text") (Duration :type "Float (double-precision)" :default 5.0) (TextColor :type "LinearColor Structure" :default (struct :`R` 1.0 :`G` 1.0 :`B` 1.0 :`A` 1.0)) (isError :type Boolean))
  (if isError
    (`KismetSystemLibrary.PrintString` null (`KismetStringLibrary.Concat_StrStr` "ERROR: " InString) true true (struct :`R` 0.489583 :`B` 0.009077 :`A` 1.0) Duration)
    (else
      (`KismetSystemLibrary.PrintString` null InString true true TextColor Duration))))

(fn `LoadSensitivity`
  (returns (Sensitivity :type "Float (double-precision)"))
  (bind _returnvalue (`GameplayStatics.DoesSaveGameExist` "SaveGame"))
  (if _returnvalue
    (bind _returnvalue_2 (`GameplayStatics.LoadGameFromSlot` "SaveGame"))
    (bind _asbp_save_game (cast `/Game/Data/BP_SaveGame` _returnvalue_2))
    (return (`/Game/Data/BP_SaveGame.UserSensitivity` _asbp_save_game))
    (else
      (return 1.0))))

(fn `LoadToken`
  (returns (Token :type String))
  (bind _returnvalue (`GameplayStatics.DoesSaveGameExist` "SaveGame"))
  (if _returnvalue
    (bind _returnvalue_2 (`GameplayStatics.LoadGameFromSlot` "SaveGame"))
    (bind _asbp_save_game (cast `/Game/Data/BP_SaveGame` _returnvalue_2))
    (return (`/Game/Data/BP_SaveGame.Token` _asbp_save_game))
    (else
      (return ""))))

(fn `RequestToApi`
  (returns (ApiUrl :type String))
  (locals (defApiUrl :type String :default "http://95.31.138.110:3000/"))
  (return (`local.defApiUrl`)))

(fn `SaveSensitivity`
  (params (UserSensitivity :type "Float (double-precision)"))
  (bind _returnvalue (`GameplayStatics.DoesSaveGameExist` "SaveGame"))
  (if _returnvalue
    (bind _returnvalue_2 (`GameplayStatics.LoadGameFromSlot` "SaveGame"))
    (bind _asbp_save_game (cast `/Game/Data/BP_SaveGame` _returnvalue_2))
    (set `/Game/Data/BP_SaveGame.UserSensitivity` UserSensitivity _asbp_save_game)
    (`GameplayStatics.SaveGameToSlot` _asbp_save_game "SaveGame")
    (else
      (bind _returnvalue_3 (`GameplayStatics.CreateSaveGameObject` "/Game/Data/BP_SaveGame.BP_SaveGame_C"))
      (set `/Game/Data/BP_SaveGame.UserSensitivity` UserSensitivity _returnvalue_3)
      (`GameplayStatics.SaveGameToSlot` _returnvalue_3 "SaveGame"))))

(fn `SaveToken`
  (params (Token :type String))
  (bind _returnvalue (`GameplayStatics.DoesSaveGameExist` "SaveGame"))
  (if _returnvalue
    (bind _returnvalue_2 (`GameplayStatics.LoadGameFromSlot` "SaveGame"))
    (bind _asbp_save_game (cast `/Game/Data/BP_SaveGame` _returnvalue_2))
    (set `/Game/Data/BP_SaveGame.Token` Token _asbp_save_game)
    (`GameplayStatics.SaveGameToSlot` _asbp_save_game "SaveGame")
    (else
      (bind _returnvalue_3 (`GameplayStatics.CreateSaveGameObject` "/Game/Data/BP_SaveGame.BP_SaveGame_C"))
      (set `/Game/Data/BP_SaveGame.Token` Token _returnvalue_3)
      (`GameplayStatics.SaveGameToSlot` _returnvalue_3 "SaveGame"))))