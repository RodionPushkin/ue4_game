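; BP_Mark is a world marker actor whose widget shows the local distance to the player character.
; Every Tick it casts the widget to W_Mark and writes the distance to player 0, divided by 100 into whole meters, into its text block.
; ToggleVisibility changes widget visibility only on the non-authority (Remote) side.
; The Sphere overlap events are empty, and the logic that would toggle visibility from them is disconnected.
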(event `self.ReceiveTick`
  (params (DeltaSeconds :type "Float (single-precision)"))
  (bind _asw_mark (cast `/Game/Blueprints/Mark/W_Mark` (`WidgetComponent.GetWidget` (`self.Widget`))))
  (bind _asbp_player_character (cast `/Game/Blueprints/Player/Game/BP_PlayerCharacter` (`GameplayStatics.GetPlayerCharacter` 0)))
  (`TextBlock.SetText` (`/Game/Blueprints/Mark/W_Mark.TextBlock_0` _asw_mark) (`KismetTextLibrary.Conv_IntToText` (/ (`KismetMathLibrary.FTrunc` (`self.GetDistanceTo` _asbp_player_character)) 100))))

(event `ToggleVisibility`
  (params (bNewVisibility :type Boolean))
  (`/Engine/EditorBlueprintResources/ActorMacros.Switch Has Authority`
    (:`Remote`
      (`SceneComponent.SetVisibility` (`self.Widget`) bNewVisibility false))))

(event `self.Sphere.OnComponentBeginOverlap`
  (params (OverlappedComponent :type "PrimitiveComponent Object Reference") (OtherActor :type "Actor Object Reference") (OtherComp :type "PrimitiveComponent Object Reference") (OtherBodyIndex :type Integer) (bFromSweep :type Boolean) (SweepResult :type "HitResult Structure (by ref)")))

(event `self.Sphere.OnComponentEndOverlap`
  (params (OverlappedComponent :type "PrimitiveComponent Object Reference") (OtherActor :type "Actor Object Reference") (OtherComp :type "PrimitiveComponent Object Reference") (OtherBodyIndex :type Integer)))

(fn `UserConstructionScript`)