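; Jetpack device that lifts the instigating player character while it has fuel.
; UseDevice sets Flying mode, burns fuel and re-fires itself on a rate timer, with a downward trace capping height above ground.
; ServerFly passes thrust to FlyMulty, which adds upward movement input and activates two Niagara effects.
; Stopping restores Falling, cuts effects and, after a delay, gradually refuels toward the class default if grounded and inactive.
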(event `self.ReceiveBeginPlay`
  (`parent.ReceiveBeginPlay`)
  (bind _asbp_player_character (cast `/Game/Blueprints/Player/Game/BP_PlayerCharacter` (`self.GetInstigator`)))
  (set `self.Character` _asbp_player_character))

(event `self.ReceiveTick`
  (params (DeltaSeconds :type "Float (single-precision)"))
  (`parent.ReceiveTick` DeltaSeconds))

(event `FlyMulty`
  (`Pawn.AddMovementInput` (`self.Character`) (`KismetMathLibrary.GetUpVector` (`KismetMathLibrary.MakeRotator` 0.0 0.0 (.yaw (`Pawn.GetControlRotation` (`self.Character`))))) (* (`self.Velocity`) (`self.ZVelocityMultiplyer`)) false)
  (`ActorComponent.Activate` (`self.Niagara1`) false)
  (`ActorComponent.Activate` (`self.Niagara`) false))

(event `ServerFly`
  (if (and (`self.Active`) (`self.CanFlyMore`))
    (`self.FlyMulty`)))

(event `self.StopUseDevice`
  (`parent.StopUseDevice`)
  (bind _asbp_player_character (cast `/Game/Blueprints/Player/Game/BP_PlayerCharacter` (`self.GetInstigator`)))
  (bind _charactermovement (`Character.CharacterMovement` _asbp_player_character))
  (`CharacterMovementComponent.SetMovementMode` _charactermovement "MOVE_Falling" 0)
  (`self.DisableFlyMulti`)
  (`KismetSystemLibrary.Delay` (`self.DurationOfGrounding`))
  (if (and (not (`NavMovementComponent.IsFalling` _charactermovement)) (not (`self.Active`)) (< (`self.Fuel`) (defaults `Object` (`GameplayStatics.GetObjectClass` self)))) :!label _label
    (`KismetSystemLibrary.Delay` (`self.RefreshRate`))
    (`/Engine/EditorBlueprintResources/StandardMacros.IncrementFloat` (`self.Fuel`)
      (:`  `
        (goto _label)))))

(event `DisableFlyMulti`
  (`ActorComponent.Deactivate` (`self.Niagara`))
  (`ActorComponent.Deactivate` (`self.Niagara1`)))

(fn `AbleToUseDevice`
  (returns (CanUse :type Boolean))
  (return (and (`parent.AbleToUseDevice`) (> (`self.Fuel`) 0.0))))

(fn `StopRateDelay`
  (bind _returnvalue (`self.GetInstigator`))
  (set `self.UseFreezedByRate` false)
  (if (`self.Active`)
    (bind _asbp_player_character (cast `/Game/Blueprints/Player/Game/BP_PlayerCharacter` _returnvalue))
    (bind (_returnvalue_x _returnvalue_y _returnvalue_z) (`KismetMathLibrary.BreakVector` (`self.K2_GetActorLocation` _asbp_player_character)))
    (bind _outhit (`KismetSystemLibrary.LineTraceSingle` (`KismetMathLibrary.MakeVector` _returnvalue_x _returnvalue_y _returnvalue_z) (`KismetMathLibrary.MakeVector` _returnvalue_x _returnvalue_y) "TraceTypeQuery1" false (`|MakeArray` _returnvalue :!type "Actor Object Reference")))
    (bind (_bblockinghit _binitialoverlap _time _distance _location _impactpoint _normal _impactnormal _physmat _hitactor _hitcomponent _hitbonename _hititem _faceindex _tracestart) (`GameplayStatics.BreakHitResult` _outhit))
    (bind (_returnvalue_x_2 _returnvalue_y_2 _returnvalue_z_2) (`KismetMathLibrary.BreakVector` (- _tracestart _location)))
    (if (<= _returnvalue_z_2 (`self.MaxFlyZ`))
      (set `self.CanFlyMore` true)
      (else
        (set `self.CanFlyMore` false)))
    (`self.UseDevice`)))

(fn `UseDevice`
  (returns (Used :type Boolean))
  (if (`self.AbleToUseDevice`)
    (set `self.Active` true)
    (bind _asbp_player_character (cast `/Game/Blueprints/Player/Game/BP_PlayerCharacter` (`self.GetInstigator`)))
    (`CharacterMovementComponent.SetMovementMode` (`Character.CharacterMovement` _asbp_player_character) "MOVE_Flying" 0)
    (`self.ServerFly`)
    (set `self.Fuel` (- (`self.Fuel`) 0.5))
    (`KismetSystemLibrary.K2_SetTimer` null "StopRateDelay" (`self.UseRate`))
    (set `self.UseFreezedByRate` true)
    (return true)
    (else
      (set `self.Active` false)
      (`self.StopUseDevice`)
      (return false))))

(fn `UserConstructionScript`
  (`parent.UserConstructionScript`))