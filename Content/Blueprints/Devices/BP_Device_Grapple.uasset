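; Grappling hook device that pulls the player character toward a surface point found by a line trace.
; UseDevice stores a hit within MaxLength and switches movement to Flying; StopUseDevice restores Falling.
; While active, Tick applies force toward the point, blended with right-axis input for steering.
; Each tick, ServerGrappling either stops within DisableLength or calls MultiGrappling, which updates cable and hook mesh visuals only on non-authority machines.
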(event `self.ReceiveBeginPlay`
  (`parent.ReceiveBeginPlay`)
  (set `self.socket` "None"))

(event `self.ReceiveTick`
  (params (DeltaSeconds :type "Float (single-precision)"))
  (bind _active (`self.Active`))
  (`parent.ReceiveTick` DeltaSeconds)
  (bind _asbp_player_character (cast `/Game/Blueprints/Player/Game/BP_PlayerCharacter` (`self.GetInstigator`)))
  (`self.ServerGrappling` _active (`self.Cable`) _asbp_player_character (`self.GrapplePoint`))
  (if _active
    (`CharacterMovementComponent.AddForce` (`Character.CharacterMovement` _asbp_player_character) (* (`KismetMathLibrary.Normal` (+ (`KismetMathLibrary.GetDirectionUnitVector` (`self.K2_GetActorLocation` _asbp_player_character) (`self.GrapplePoint`)) (* (* (`self.GetActorRightVector` _asbp_player_character) (`self.GetInputAxisValue`)) 0.5))) (`self.strength`)))))

(event `ServerGrappling`
  (params (Condition :type Boolean) (Cable :type "CableComponent Object Reference") (Character :type "/Game/Blueprints/Player/Game/BP_PlayerCharacter Object Reference") (Location :type "Vector Structure"))
  (if (<= (`KismetMathLibrary.Vector_Distance` Location (`self.K2_GetActorLocation` Character)) (`self.DisableLength`))
    (`self.StopUseDevice`)
    (else
      (`self.MultiGrappling` Condition Cable Character Location))))

(event `MultiGrappling`
  (params (Condition :type Boolean) (Cable :type "CableComponent Object Reference") (Character :type "/Game/Blueprints/Player/Game/BP_PlayerCharacter Object Reference") (Location :type "Vector Structure"))
  (bind _returnvalue (`KismetMathLibrary.InverseTransformLocation` (`self.GetTransform` Character) Location))
  (`/Engine/EditorBlueprintResources/ActorMacros.Switch Has Authority`
    (:`Remote`
      (if Condition
        (`SceneComponent.SetVisibility` Cable true false)
        (`SceneComponent.SetVisibility` (`self.StaticMesh1`) true false)
        (set `CableComponent.EndLocation` _returnvalue Cable)
        (`SceneComponent.K2_SetRelativeLocation` (`self.StaticMesh1`) _returnvalue false true)
        (else
          (`SceneComponent.SetVisibility` Cable false false)
          (`SceneComponent.SetVisibility` (`self.StaticMesh1`) false false))))))

(event `MultiGrapple`
  (params (Character :type "Character Object Reference") (GrapplePoint :type "Vector Structure") (Cable :type "CableComponent Object Reference") (Target :type "/Game/Blueprints/Player/Game/BP_PlayerCharacter Object Reference")))

(event `ServerGrapple`
  (params (Character :type "Character Object Reference") (GrapplePoint :type "Vector Structure") (Cable :type "CableComponent Object Reference") (Target :type "/Game/Blueprints/Player/Game/BP_PlayerCharacter Object Reference")))

(fn `AbleToUseDevice`
  (returns (CanUse :type Boolean))
  (return (`parent.AbleToUseDevice`)))

(fn `StopUseDevice`
  (`parent.StopUseDevice`)
  (bind _asbp_player_character (cast `/Game/Blueprints/Player/Game/BP_PlayerCharacter` (`self.GetInstigator`)))
  (`CharacterMovementComponent.SetMovementMode` (`Character.CharacterMovement` _asbp_player_character) "MOVE_Falling" 0)
  (set `self.Active` false))

(fn `UseDevice`
  (returns (Used :type Boolean))
  (if (`self.AbleToUseDevice`)
    (bind _asbp_player_character (cast `/Game/Blueprints/Player/Game/BP_PlayerCharacter` (`self.GetInstigator`)))
    (bind _returnvalue (`SceneComponent.K2_GetComponentLocation` (`/Game/Blueprints/Player/Game/BP_PlayerCharacter.Camera` _asbp_player_character)))
    (bind (_outhit _returnvalue_2) (`KismetSystemLibrary.LineTraceSingle` _returnvalue (+ _returnvalue (* (`self.GetActorForwardVector` (`self.GetOwner`)) 10000.0)) "TraceTypeQuery1" false (`|MakeArray` _asbp_player_character :!type "Actor Object Reference")))
    (if _returnvalue_2
      (bind (_bblockinghit _binitialoverlap _time _distance _location _impactpoint) (`GameplayStatics.BreakHitResult` _outhit))
      (if (< _distance (`self.MaxLength`))
        (set `self.GrapplePoint` _impactpoint)
        (set `self.Active` true)
        (`CharacterMovementComponent.SetMovementMode` (`Character.CharacterMovement` _asbp_player_character) "MOVE_Flying" 0)
        (return true)
        (else
          (return false))))
    (else
      (return false))))

(fn `UserConstructionScript`
  (`parent.UserConstructionScript`))