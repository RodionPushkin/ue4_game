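; BP_Device is an Actor Blueprint that provides a minimal use and stop interface for devices.
; UseDevice returns whether AbleToUseDevice passes, which is true unless the UseFreezedByRate flag is set.
; StopUseDevice clears the Active flag, while nothing here sets Active or the rate freeze, and the event graph and construction script are empty.
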(fn `AbleToUseDevice`
  (returns (CanUse :type Boolean))
  (return (not (`self.UseFreezedByRate`))))

(fn `StopUseDevice`
  (set `self.Active` false)
  (return))

(fn `UseDevice`
  (returns (Used :type Boolean))
  (if (`self.AbleToUseDevice`)
    (return true)
    (else
      (return false))))

(fn `UserConstructionScript`)