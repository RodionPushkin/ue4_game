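; Player controller that manages the in-game screen, escape menu and settings widgets.
; ESC and Statistics inputs share one handler that steps between game screen and escape menu, or from settings back to the menu.
; Switching between game and menu also sets the cursor, input mode and character's CanMove flag.
; Toggle events create or remove each widget, whose validity serves as menu state, and DisableMovement disables controller input.
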(event `InputAction|Statistics`
  (params (Key :type "Key Structure"))
  (bind (_sizex _sizey) (`self.GetViewportSize`))
  (bind _wsettings (`self.WSettings`))
  (bind _wesc (`self.WEsc`))
  ;[1 1 1] Open and close escape widget
  (:`Pressed`
    (`/Engine/EditorBlueprintResources/StandardMacros.IsValid` (`self.WGame`) :!label _label
      (:`Is Valid`
        (`self.ToggleEsc` true)
        (`self.ToggleGameScreen` false)
        (`self.SetMouseLocation` (/ _sizex 2) (/ _sizey 2))
        (set `self.bShowMouseCursor` true)
        (bind _asbp_player_character (cast `/Game/Blueprints/Player/Game/BP_PlayerCharacter` (`GameplayStatics.GetPlayerCharacter` 0)))
        (set `/Game/Blueprints/Player/Game/BP_PlayerCharacter.CanMove` false _asbp_player_character)
        (`/Engine/EditorBlueprintResources/StandardMacros.IsValid` _wsettings
          (:`Is Valid`
            (`WidgetBlueprintLibrary.SetInputMode_GameAndUIEx` self _wsettings "DoNotLock" false))
          (:`Is Not Valid`
            (`/Engine/EditorBlueprintResources/StandardMacros.IsValid` _wesc
              (:`Is Valid`
                (`WidgetBlueprintLibrary.SetInputMode_GameAndUIEx` self _wesc "DoNotLock" false))))))
      (:`Is Not Valid`
        (`/Engine/EditorBlueprintResources/StandardMacros.IsValid` (`self.WEsc`)
          (:`Is Valid`
            (`self.ToggleGameScreen` true)
            (`self.ToggleEsc` false)
            (set `self.bShowMouseCursor` false)
            (bind _asbp_player_character_2 (cast `/Game/Blueprints/Player/Game/BP_PlayerCharacter` (`GameplayStatics.GetPlayerCharacter` 0)))
            (set `/Game/Blueprints/Player/Game/BP_PlayerCharacter.CanMove` true _asbp_player_character_2)
            (`WidgetBlueprintLibrary.SetFocusToGameViewport`)
            (`WidgetBlueprintLibrary.SetInputMode_GameOnly` self))
          (:`Is Not Valid`
            (`/Engine/EditorBlueprintResources/StandardMacros.IsValid` (`self.WSettings`)
              (:`Is Valid`
                (`self.ToggleGameScreen` false)
                (`self.ToggleEsc` true)
                (`self.ToggleSettings` false)))))))))

(event `InputAction|ESC`
  (params (Key :type "Key Structure"))
  ;[1 1 1] Open and close escape widget
  (:`Pressed`
    (goto _label)))

(event `ToggleSettings`
  (params (input :type Boolean))
  (bind _wsettings (`self.WSettings`))
  (if input
    (bind _returnvalue (`|CreateWidget` "/Game/UI/Settings/W_Settings.W_Settings_C"))
    (set `self.WSettings` _returnvalue)
    (`UserWidget.AddToViewport` (`self.WSettings`) 0)
    (else
      (`/Engine/EditorBlueprintResources/StandardMacros.IsValid` _wsettings
        (:`Is Valid`
          (`Widget.RemoveFromParent` _wsettings)
          (set `self.WSettings` null))))))

(event `ToggleEsc`
  (params (Input :type Boolean))
  (bind _wesc (`self.WEsc`))
  (if Input
    (bind _returnvalue (`|CreateWidget` "/Game/UI/InGame/W_GameEsc.W_GameEsc_C"))
    (set `self.WEsc` _returnvalue)
    (`UserWidget.AddToViewport` (`self.WEsc`) 0)
    (else
      (`/Engine/EditorBlueprintResources/StandardMacros.IsValid` _wesc
        (:`Is Valid`
          (`Widget.RemoveFromParent` _wesc)
          (set `self.WEsc` null))))))

(event `ToggleGameScreen`
  (params (Input :type Boolean))
  (bind _wgame (`self.WGame`))
  (if Input
    (bind _returnvalue (`|CreateWidget` "/Game/UI/InGame/W_GameScreen.W_GameScreen_C"))
    (set `self.WGame` _returnvalue)
    (`UserWidget.AddToViewport` (`self.WGame`) 0)
    (else
      (`/Engine/EditorBlueprintResources/StandardMacros.IsValid` _wgame
        (:`Is Valid`
          (`Widget.RemoveFromParent` _wgame)
          (set `self.WGame` null))))))

(fn `DisableMovement`
  (`self.DisableInput` null))

(fn `UserConstructionScript`)