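; Menu player controller that manages the main menu, escape menu and settings widgets.
; The ESC and Statistics inputs share one chain: main menu switches to escape menu, escape menu back to main menu, and settings to escape menu.
; Toggle events create each widget and add it to the viewport, or remove it and clear its reference, so reference validity tracks the open screen.
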(event `InputAction|Statistics`
  (params (Key :type "Key Structure"))
  ;[1 1 1] Open and close escape widget
  (:`Pressed`
    (`/Engine/EditorBlueprintResources/StandardMacros.IsValid` (`self.WMenu`) :!label _label
      (:`Is Valid`
        (`self.ToggleEsc` true)
        (`self.ToggleMenu` false))
      (:`Is Not Valid`
        (`/Engine/EditorBlueprintResources/StandardMacros.IsValid` (`self.WEsc`)
          (:`Is Valid`
            (`self.ToggleMenu` true)
            (`self.ToggleEsc` false))
          (:`Is Not Valid`
            (`/Engine/EditorBlueprintResources/StandardMacros.IsValid` (`self.WSettings`)
              (:`Is Valid`
                (`self.ToggleMenu` false)
                (`self.ToggleEsc` true)
                (`self.ToggleSettings` false)))))))))

(event `InputAction|ESC`
  (params (Key :type "Key Structure"))
  ;[1 1 1] Open and close escape widget
  (:`Pressed`
    (goto _label)))

(event `ToggleSettings`
  (params (input :type Boolean))
  (bind _wsettings (`self.WSettings`))
  (if input
    (bind _returnvalue (`|CreateWidget` "/Game/UI/Settings/W_Settings.W_Settings_C"))
    (set `self.WSettings` _returnvalue)
    (`UserWidget.AddToViewport` (`self.WSettings`) 0)
    (else
      (`/Engine/EditorBlueprintResources/StandardMacros.IsValid` _wsettings
        (:`Is Valid`
          (`Widget.RemoveFromParent` _wsettings)
          (set `self.WSettings` null))))))

(event `ToggleEsc`
  (params (Input :type Boolean))
  (bind _wesc (`self.WEsc`))
  (if Input
    (bind _returnvalue (`|CreateWidget` "/Game/UI/Menu/W_MenuEsc.W_MenuEsc_C"))
    (set `self.WEsc` _returnvalue)
    (`UserWidget.AddToViewport` (`self.WEsc`) 0)
    (else
      (`/Engine/EditorBlueprintResources/StandardMacros.IsValid` _wesc
        (:`Is Valid`
          (`Widget.RemoveFromParent` _wesc)
          (set `self.WEsc` null))))))

(event `ToggleMenu`
  (params (Input :type Boolean))
  (bind _wmenu (`self.WMenu`))
  (if Input
    (bind _returnvalue (`|CreateWidget` "/Game/UI/Menu/W_Menu.W_Menu_C"))
    (set `self.WMenu` _returnvalue)
    (`UserWidget.AddToViewport` (`self.WMenu`) 0)
    (else
      (`/Engine/EditorBlueprintResources/StandardMacros.IsValid` _wmenu
        (:`Is Valid`
          (`Widget.RemoveFromParent` _wmenu)
          (set `self.WMenu` null))))))

(fn `UserConstructionScript`)