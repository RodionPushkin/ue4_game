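; Menu character Blueprint that shows the player's nickname on its attached widget.
; BeginPlay loads and applies game user settings, then, only without authority, sends the saved token to the user API through VaRest.
; The callback writes the returned nickname into W_Nickname, or prints the error and opens M_Loading if no user comes back.
; A separate PlaySound event plays a given sound at a location.
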(event `PlaySound`
  (params (Location :type "Vector Structure") (Sound :type "SoundBase Object Reference"))
  (`GameplayStatics.PlaySoundAtLocation` Sound Location (struct) 1.0 1.0 0.0 null null null))

(event `self.ReceiveBeginPlay`
  (bind _returnvalue (subsystem `VaRestSubsystem`))
  (bind _returnvalue_2 (`GameUserSettings.GetGameUserSettings`))
  (`GameUserSettings.LoadSettings` _returnvalue_2 false)
  (`GameUserSettings.ApplySettings` _returnvalue_2 true)
  (`/Engine/EditorBlueprintResources/ActorMacros.Switch Has Authority`
    (:`Remote`
      (bind _returnvalue_3 (`VaRestSubsystem.DecodeJsonObject` _returnvalue (`KismetStringLibrary.Concat_StrStr` "{\"token\": \"" (`/Game/Blueprints/BP_CustomFunctions.LoadToken`) "\"}")))
      (`VaRestSubsystem.CallURL` _returnvalue (`KismetStringLibrary.Concat_StrStr` (`/Game/Blueprints/BP_CustomFunctions.RequestToApi`) "user") "PUT" "json" _returnvalue_3 (delegate `CustomEvent_0`)))))

(event `CustomEvent_0`
  (params (Request :type "VaRestRequestJSON Object Reference"))
  (bind _returnvalue (`VaRestRequestJSON.GetResponseObject` Request))
  (bind _returnvalue_2 (`VaRestJsonObject.GetField` _returnvalue "User"))
  (`/Engine/EditorBlueprintResources/StandardMacros.IsValid` _returnvalue_2
    (:`Is Valid`
      (bind _returnvalue_3 (`VaRestJsonValue.AsObject` _returnvalue_2))
      (bind _asw_nickname (cast `/Game/UI/W_Nickname` (`WidgetComponent.GetWidget` (`self.Widget`))))
      (`TextBlock.SetText` (`/Game/UI/W_Nickname.TextBlock_33` _asw_nickname) (`KismetTextLibrary.Conv_StringToText` (`VaRestJsonObject.GetStringField` _returnvalue_3 "Nickname"))))
    (:`Is Not Valid`
      (`KismetSystemLibrary.PrintString` (`VaRestJsonObject.GetStringField` _returnvalue "Error"))
      (`GameplayStatics.OpenLevel` "M_Loading"))))

(fn `UserConstructionScript`)