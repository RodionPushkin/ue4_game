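; C_Gordon is a Blueprint that creates the W_Gordon widget and starts its MediaSound when play begins.
; BeginPlay creates the widget for player controller 0 and stores it in the WGordon variable.
; A RepNotify on that variable adds the widget to the viewport, while the AddToViewport call left in the event graph is disconnected.
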(event `self.ReceiveBeginPlay`
  (bind _returnvalue (`|CreateWidget` "/Game/Umg/Gordon/W_Gordon.W_Gordon_C" (`GameplayStatics.GetPlayerController` 0)))
  (set `self.W_gordon` _returnvalue)
  (`SynthComponent.Start` (`self.MediaSound`)))

(fn `OnRep_W_gordon`
  (if (not (== (`self.W_gordon`) null))
    (`UserWidget.AddToViewport` (`self.W_gordon`) 0)))

(fn `UserConstructionScript`)