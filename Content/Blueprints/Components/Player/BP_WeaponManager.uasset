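; Player component that manages the character's weapons: creation, slot storage and the currently selected weapon.
; CreateWeapon spawns a weapon owned by the controller, files it by type into main, second, melee, special or grenade storage, and attaches it to the character.
; SelectWeapon only sets CurrentWeapon, whose RepNotify attaches it to the visible mesh's SKT_Weapon socket on non-server instances only.
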(event `self.ReceiveBeginPlay`
  (bind _asbp_player_character (cast `/Game/Blueprints/Player/Game/BP_PlayerCharacter` (`self.GetOwner`)))
  (set `self.Character` _asbp_player_character))

(fn `CreateWeapon`
  (params (Class :type "Actor Class Reference"))
  (returns (Weapon :type "/Game/Blueprints/Weapons/BP_Weapon Object Reference"))
  (locals (L_Weapon :type "/Game/Blueprints/Weapons/BP_Weapon Object Reference"))
  (bind _character (`self.Character`))
  (bind _l_weapon (`local.L_Weapon`))
  (bind _returnvalue (`|SpawnActorFromClass` Class (`KismetMathLibrary.MakeTransform` (0.0 0.0 0.0)) "AlwaysSpawn" "OverrideRootScale" (`Pawn.GetController` _character) _character))
  (bind _asbp_weapon (cast `/Game/Blueprints/Weapons/BP_Weapon` _returnvalue))
  (set `local.L_Weapon` _asbp_weapon)
  (switch `/Game/Data/E_Weapons` (`/Game/Blueprints/Weapons/BP_Weapon.WeaponType` _asbp_weapon)
    (:`NewEnumerator0`
      (set `self.MainWeapon` _l_weapon))
    (:`NewEnumerator1`
      (set `self.SesondWeapon` _l_weapon))
    (:`NewEnumerator3`
      (`KismetArrayLibrary.Array_Add` (`self.Specials`) _l_weapon))
    (:`NewEnumerator4`
      (`KismetArrayLibrary.Array_Add` (`self.Grenades`) _l_weapon))
    (:`NewEnumerator5`
      (set `self.MeleeWeapon` _l_weapon)))
  (`Actor.K2_AttachToActor` (`local.L_Weapon`) (`self.Character`) "None" "SnapToTarget" "SnapToTarget" "KeepRelative" true)
  (return (`local.L_Weapon`)))

(fn `OnRep_CurrentWeapon`
  (if (not (`KismetSystemLibrary.IsServer`))
    (`Actor.K2_AttachToComponent` (`self.CurrentWeapon`) (`/Game/Blueprints/Player/Game/BP_PlayerCharacter.GetVisibleMesh` (`self.Character`)) "SKT_Weapon" "KeepRelative" "KeepRelative" "KeepRelative" true)))

(fn `SelectWeapon`
  (params (CurrentWeapon :type "/Game/Blueprints/Weapons/BP_Weapon Object Reference"))
  (set `self.CurrentWeapon` CurrentWeapon))