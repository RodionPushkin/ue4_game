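; BP_DeviceManager is a player component that spawns and tracks the device held by BP_PlayerCharacter.
; CreateDevice spawns a BP_Device owned by the character's controller and snaps it to the character at the device's socket.
; SelectDevice sets the replicated current Device, whose OnRep attaches it to the character's visible mesh on non-server machines.
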(event `self.ReceiveBeginPlay`
  (bind _asbp_player_character (cast `/Game/Blueprints/Player/Game/BP_PlayerCharacter` (`self.GetOwner`)))
  (set `self.Character` _asbp_player_character))

(fn `CreateDevice`
  (params (Class :type "Actor Class Reference"))
  (returns (Device :type "/Game/Blueprints/Devices/BP_Device Object Reference"))
  (locals (L_Device :type "/Game/Blueprints/Devices/BP_Device Object Reference"))
  (bind _character (`self.Character`))
  (bind _l_device (`local.L_Device`))
  (bind _returnvalue (`|SpawnActorFromClass` Class (`KismetMathLibrary.MakeTransform` (0.0 0.0 0.0)) "AlwaysSpawn" "OverrideRootScale" (`Pawn.GetController` _character) _character))
  (bind _asbp_device (cast `/Game/Blueprints/Devices/BP_Device` _returnvalue))
  (set `local.L_Device` _asbp_device)
  (`Actor.K2_AttachToActor` _l_device (`self.Character`) (`/Game/Blueprints/Devices/BP_Device.socket` _l_device) "SnapToTarget" "SnapToTarget" "KeepRelative" true)
  (return (`local.L_Device`)))

(fn `OnRep_Device`
  (bind _device (`self.Device`))
  (if (not (`KismetSystemLibrary.IsServer`))
    (`Actor.K2_AttachToComponent` _device (`/Game/Blueprints/Player/Game/BP_PlayerCharacter.GetVisibleMesh` (`self.Character`)) (`/Game/Blueprints/Devices/BP_Device.socket` _device) "KeepRelative" "KeepRelative" "KeepRelative" true)))

(fn `SelectDevice`
  (params (Device :type "/Game/Blueprints/Devices/BP_Device Object Reference"))
  (set `self.Device` Device))