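; Player component that manages a single world mark, keeping a reference to the current BP_Mark actor.
; SpawnMark destroys any existing mark, then line-traces on Visibility from the character's camera along the controller's forward vector.
; On a hit it spawns a mark there, owned by the controller and instigated by the character.
; A separate Spawn function places a mark at a supplied location without clearing the previous one.
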(event `self.ReceiveBeginPlay`
  (bind _asbp_player_character (cast `/Game/Blueprints/Player/Game/BP_PlayerCharacter` (`self.GetOwner`)))
  (set `self.Character` _asbp_player_character))

(fn `DestroyMark`
  (`Actor.K2_DestroyActor` (`self.CurrentMark`))
  (set `self.CurrentMark` null))

(fn `Spawn`
  (params (`Spawn Transform Location` :type "Vector Structure") (Instigator :type "Pawn Object Reference") (Owner :type "Actor Object Reference"))
  (bind _returnvalue (`|SpawnActorFromClass` "/Game/Blueprints/Mark/BP_Mark.BP_Mark_C" (`KismetMathLibrary.MakeTransform` `Spawn Transform Location`) "AlwaysSpawn" "OverrideRootScale" Owner Instigator))
  (set `self.CurrentMark` _returnvalue))

(fn `SpawnMark`
  (params (Character :type "/Game/Blueprints/Player/Game/BP_PlayerCharacter Object Reference"))
  (bind _returnvalue (`Pawn.GetController` Character))
  (bind _returnvalue_2 (`SceneComponent.K2_GetComponentLocation` (`/Game/Blueprints/Player/Game/BP_PlayerCharacter.Camera` Character)))
  (`/Engine/EditorBlueprintResources/StandardMacros.IsValid` (`self.CurrentMark`)
    (:`Is Valid`
      (`self.DestroyMark`))
    (:`Is Not Valid`
      _))
  (bind (_outhit _returnvalue_3) (`KismetSystemLibrary.LineTraceSingle` _returnvalue_2 (+ _returnvalue_2 (* (`Actor.GetActorForwardVector` _returnvalue) 10000.0)) "TraceTypeQuery1"))
  (if _returnvalue_3
    (bind _returnvalue_4 (`|SpawnActorFromClass` "/Game/Blueprints/Mark/BP_Mark.BP_Mark_C" (`KismetMathLibrary.MakeTransform` (`.Location` (`GameplayStatics.BreakHitResult` _outhit))) "AlwaysSpawn" "OverrideRootScale" _returnvalue Character))
    (set `self.CurrentMark` _returnvalue_4)))