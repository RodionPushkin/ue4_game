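; Player health component that tracks shield, health and death for BP_PlayerCharacter.
; On BeginPlay the server binds to the owner's any-damage event and passes incoming damage to ApplyDamage.
; Damage drains the shield, health takes half while the remaining shield is at least 50 and full otherwise, and zero health sets Dead.
; The Dead RepNotify fires the character-dead call and disables the character's movement.
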(event `self.ReceiveBeginPlay`
  (bind _asbp_player_character (cast `/Game/Blueprints/Player/Game/BP_PlayerCharacter` (`self.GetOwner`)))
  (bind _output_get (set `self.Character` _asbp_player_character))
  (if (`KismetSystemLibrary.IsServer`)
    (add `Actor.OnTakeAnyDamage` _output_get (delegate `OnPlayerTakeAnyDamage`))))

(event `OnPlayerTakeAnyDamage`
  (params (DamagedActor :type "Actor Object Reference") (Damage :type "Float (double-precision)") (DamageType :type "DamageType Object Reference") (InstigatedBy :type "Controller Object Reference") (DamageCauser :type "Actor Object Reference"))
  (`self.ApplyDamage` Damage))

(fn `ApplyDamage`
  (params (Damage :type "Float (double-precision)"))
  (bind _output_get (set `self.Shield` (- (`self.Shield`) Damage)))
  (if (>= _output_get 50.0)
    (set `self.Health` (- (`self.Health`) (/ Damage 2.0)))
    (else
      (set `self.Health` (- (`self.Health`) Damage))))
  (if (<= (`self.Health`) 0.0)
    (set `self.Dead` true)
    (set `self.Health` 0.0))
  (if (<= (`self.Shield`) 0.0)
    (set `self.Shield` 0.0)))

(fn `OnRep_Dead`
  (bind _character (`self.Character`))
  (if (`self.Dead`)
    (`self.CharacterDead`)
    (set `/Game/Blueprints/Player/Game/BP_PlayerCharacter.CanMove` false _character)
    (`CharacterMovementComponent.DisableMovement` (`Character.CharacterMovement` _character))
    (if (`KismetSystemLibrary.IsServer`)
      (`KismetSystemLibrary.PrintString` "вот и помер дед максим"))))